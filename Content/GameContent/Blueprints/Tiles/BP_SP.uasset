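; BP_SP is a Rabbit Smasher "SP" point that the player closes by standing inside its box until its Health fills.
; While the player overlaps, Tick adds Health per frame up to a cap, then increments the game mode's ClosedSP, with a flag preventing repeat counts until refilling resumes.
; Damage lowers Health without decrementing ClosedSP, and a UW_SPHealth widget component mirrors the value as progress.
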(event `self.ReceiveAnyDamage`
  (params (Damage :type "Float (single-precision)") (DamageType :type "DamageType Object Reference") (InstigatedBy :type "Controller Object Reference") (DamageCauser :type "Actor Object Reference"))
  (bind _health (`self.Health`))
  (`KismetSystemLibrary.PrintString` "DamageTaken")
  (if (> _health 0.0)
    (bind _output_get (set `self.Health` (- _health Damage)))
    (set `/Game/Aditya/UW_SPHealth.SP_Progress` _output_get (`self.As UW SPHealth`))))

(event `self.ReceiveBeginPlay`
  (bind _asgm_rabbit_smasher (cast `/Game/GameContent/Blueprints/GM_RabbitSmasher` (`GameplayStatics.GetGameMode`)))
  (set `self.As GM Rabbit Smasher` _asgm_rabbit_smasher)
  (bind _asuw_sphealth (cast `/Game/Aditya/UW_SPHealth` (`WidgetComponent.GetUserWidgetObject` (`self.Widget`))))
  (bind _output_get (set `self.As UW SPHealth` _asuw_sphealth))
  (set `/Game/Aditya/UW_SPHealth.SP_Progress` (`self.Health`) _output_get))

(event `self.Box.OnComponentBeginOverlap`
  (params (OverlappedComponent :type "PrimitiveComponent Object Reference") (OtherActor :type "Actor Object Reference") (OtherComp :type "PrimitiveComponent Object Reference") (OtherBodyIndex :type Integer) (bFromSweep :type Boolean) (SweepResult :type "HitResult Structure (by ref)"))
  (if (== OtherActor (`GameplayStatics.GetPlayerCharacter` 0))
    (set `self.PlayerInRange` true)
    (`KismetSystemLibrary.PrintString` "enetered")))

(event `self.Box.OnComponentEndOverlap`
  (params (OverlappedComponent :type "PrimitiveComponent Object Reference") (OtherActor :type "Actor Object Reference") (OtherComp :type "PrimitiveComponent Object Reference") (OtherBodyIndex :type Integer))
  (if (== OtherActor (`GameplayStatics.GetPlayerCharacter` 0))
    (set `self.PlayerInRange` false)
    (`KismetSystemLibrary.PrintString` "exited")))

(event `self.ReceiveTick`
  (params (DeltaSeconds :type "Float (single-precision)"))
  (bind _as_gm_rabbit_smasher (`self.As GM Rabbit Smasher`))
  (bind _health (`self.Health`))
  (if (`self.PlayerInRange`)
    (if (< _health 100.0)
      (set `self.temp` true)
      (bind _result (`/Engine/EditorBlueprintResources/StandardMacros.IncrementFloat` _health)
        (:`  `
          (bind _output_get (set `self.Health` _result))
          (set `/Game/Aditya/UW_SPHealth.SP_Progress` _output_get (`self.As UW SPHealth`))))
      (elif (`self.temp`)
        (set `self.temp` false)
        (bind _result_2 (`/Engine/EditorBlueprintResources/StandardMacros.IncrementInt` (`/Game/GameContent/Blueprints/GM_RabbitSmasher.Closed_SP` _as_gm_rabbit_smasher))
          (:`  `
            (set `/Game/GameContent/Blueprints/GM_RabbitSmasher.Closed_SP` _result_2 _as_gm_rabbit_smasher)))))))

(fn `UserConstructionScript`)