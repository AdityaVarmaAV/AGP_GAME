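; BP_10x10TileBase is a base tile Blueprint that alerts the player when it is under attack.
; Its widget component starts hidden, and the Underattack! event shows it, plays the UI_UnderAttack animation and sounds a 2D alarm.
; The widget hides again after a short delay, while a DoOnce gate resets on a longer delay to throttle repeated alerts.
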(event `self.ReceiveBeginPlay`
  (`Widget.SetVisibility` (`WidgetComponent.GetWidget` (`self.Widget`)) "Hidden"))

(event `Under attack!`
  (bind _returnvalue (`WidgetComponent.GetWidget` (`self.Widget`)))
  (`/Engine/EditorBlueprintResources/StandardMacros.DoOnce` false :!label _label
    (:`Completed`
      (`Widget.SetVisibility` _returnvalue "Visible")
      (bind _asui_under_attack (cast `/Game/GameContent/Blueprints/Tiles/UI_UnderAttack` _returnvalue)
        (:`then`
          (`/Game/GameContent/Blueprints/Tiles/UI_UnderAttack.PlayAnimation uwu` _asui_under_attack)
          (`GameplayStatics.PlaySound2D` "/Game/GameContent/SoundEffects/alarming-39985.alarming-39985" 1.0 1.0 0.0 null null)
          (`|ExecutionSequence`
            (:`then_0`
              (`KismetSystemLibrary.Delay` 15.0)
              (goto _label :!via `Reset`))
            (:`then_1`
              (`KismetSystemLibrary.Delay` 3.0)
              (`Widget.SetVisibility` _returnvalue "Hidden"))))
        (:`CastFailed`
          (`KismetSystemLibrary.PrintString` "Cast failed"))))))

(fn `UserConstructionScript`)