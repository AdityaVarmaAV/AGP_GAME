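; BP_Crop is a destructible carrot or lettuce crop in the Rabbit Smasher game mode, with its mesh chosen by CropType in the construction script.
; Any damage lowers Health and plays a hurt effect and sound at the crop.
; A surviving crop calls UnderAttack on its parent 10x10 tile actor.
; At zero health it leaves the game mode's crop list, triggers a loss check and destroys itself.
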(event `self.ReceiveBeginPlay`)

(event `self.ReceiveAnyDamage`
  (params (Damage :type "Float (single-precision)") (DamageType :type "DamageType Object Reference") (InstigatedBy :type "Controller Object Reference") (DamageCauser :type "Actor Object Reference"))
  (bind _returnvalue (`self.K2_GetActorLocation`))
  (bind _output_get (set `self.Health` (- (`self.Health`) Damage)))
  (`NiagaraFunctionLibrary.SpawnSystemAtLocation` "/Game/GameContent/VFX/VX_PlantHurt.VX_PlantHurt" _returnvalue (struct :`Pitch` 90.0))
  (`GameplayStatics.PlaySoundAtLocation` "/Game/GameContent/SoundEffects/carrotnom-92106.carrotnom-92106" _returnvalue (struct) 1.0 1.0 0.0 "/Game/GameContent/SoundEffects/AttenSetting.AttenSetting" null null null)
  (if (<= _output_get 0.0)
    (bind _asgm_rabbit_smasher (cast `/Game/GameContent/Blueprints/GM_RabbitSmasher` (`GameplayStatics.GetGameMode`)))
    (`KismetArrayLibrary.Array_RemoveItem` (`/Game/GameContent/Blueprints/GM_RabbitSmasher.AllCropsReference` _asgm_rabbit_smasher) self)
    (`/Game/GameContent/Blueprints/GM_RabbitSmasher.Check Loss` _asgm_rabbit_smasher)
    (`self.K2_DestroyActor`)
    (else
      (bind _asbp_10x_10tile_base (cast `/Game/GameContent/Blueprints/Tiles/BP_10x10TileBase` (`self.GetParentActor`)))
      (`/Game/GameContent/Blueprints/Tiles/BP_10x10TileBase.Under attack!` _asbp_10x_10tile_base))))

(fn `UserConstructionScript`
  (`StaticMeshComponent.SetStaticMesh` (`self.StaticMesh`) (select `/Game/GameContent/Blueprints/Crop/E_CropTypes` (`self.CropType`) :`NewEnumerator0` "/Game/PolygonFarm/Meshes/Plants/SM_Prop_Carrot_01.SM_Prop_Carrot_01" :`NewEnumerator1` "/Game/PolygonFarm/Meshes/Plants/SM_Prop_Lettuce_01_L.SM_Prop_Lettuce_01_L" :!type "StaticMesh Object Reference")))