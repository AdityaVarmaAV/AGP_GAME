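; BP_Rabbit is an AI rabbit actor that supplies the creature's hop motion, sounds and death effects.
; On BeginPlay, a timeline moves the static mesh vertically to suggest hopping, while a self-looping delay repeatedly plays the walk cue at the actor's location.
; When the actor is destroyed, it spawns a blood explosion effect and plays an attenuated death sound at its position.
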(event `self.ReceiveDestroyed`
  (`NiagaraFunctionLibrary.SpawnSystemAtLocation` "/Game/GameContent/VFX/VX_BloodExplosion.VX_BloodExplosion" (`self.K2_GetActorLocation`))
  (`GameplayStatics.PlaySoundAtLocation` "/Game/GameContent/SoundEffects/RabbitDeath.RabbitDeath" (`self.K2_GetActorLocation`) (struct) 1.2 1.0 0.0 "/Game/GameContent/SoundEffects/AttenSetting.AttenSetting" null null null))

(event `self.ReceiveBeginPlay`
  (`|ExecutionSequence`
    (:`then_0`
      (bind (_direction _newtrack_0) (`Timeline|Timeline_0` :!via `PlayFromStart`)
        (:`Update`
          (`SceneComponent.K2_SetRelativeLocation` (`self.StaticMesh`) (`KismetMathLibrary.MakeVector` 0.0 0.0 (`KismetMathLibrary.Lerp` 10.0 40.0 _newtrack_0)) false false))))
    (:`then_1`
      (`KismetSystemLibrary.Delay` 0.6 :!label _label)
      (`GameplayStatics.PlaySoundAtLocation` "/Game/GameContent/SoundEffects/RabbitWalk_Cue.RabbitWalk_Cue" (`self.K2_GetActorLocation`) (struct) 1.0 1.0 0.0 "/Game/GameContent/SoundEffects/AttenSetting.AttenSetting" null null null)
      (goto _label))))

(fn `UserConstructionScript`)