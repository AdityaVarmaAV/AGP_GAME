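; Wave controller for the Rabbit Smasher game mode that runs enemy waves and triggers victory after the last one.
; Each wave's type-to-count map expands into a shuffled queue, which a looping timer feeds to random BP_Spawner actors.
; Checkifalldead? advances the wave when the queue is empty and exactly one "Enemy"-tagged actor remains.
; A DoOnce guards the transition, which resets the spawn interval and pauses before spawning resumes.
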(event `self.ReceiveBeginPlay`
  ;[1 1 1] Turning the first wave into an array
  (`KismetSystemLibrary.DelayUntilNextTick`)
  (bind _outactors (`GameplayStatics.GetAllActorsOfClass` "/Game/GameContent/AI/RabbitBlueprints/BP_Spawner.BP_Spawner_C"))
  (set `self.Spawners` _outactors)
  (`self.SetupWaveContents` (`self.Current wave`))
  (`self.Start Spawning`)
  (`KismetSystemLibrary.PrintString` "Wave 1 begin" true true (struct :`R` 1.0 :`G` 1.0 :`A` 1.0)))

(event `self.ReceiveTick`
  (params (DeltaSeconds :type "Float (single-precision)"))
  (`KismetSystemLibrary.PrintString` (`KismetStringLibrary.Conv_IntToString` (`self.Current wave`)) true true (struct :`G` 1.0 :`B` 0.294202 :`A` 1.0) 0.0))

(event `Start Spawning`
  (bind _returnvalue (`KismetSystemLibrary.K2_SetTimerDelegate` (delegate `Spawn Enemy`) (`self.Delay between spawns`) true))
  (set `self.SpawningTimer` _returnvalue))

(event `Spawn Enemy`
  (bind _current_wave_enemies (`self.Current wave enemies`))
  (if (> (`KismetArrayLibrary.Array_Length` _current_wave_enemies) 0)
    (`/Game/GameContent/AI/RabbitBlueprints/BP_Spawner.Spawn enemy` (`KismetArrayLibrary.Array_Random` (`self.Spawners`)) (`|GetArrayItem` _current_wave_enemies))
    (`KismetArrayLibrary.Array_Remove` _current_wave_enemies)
    (set `self.Delay between spawns` (+ (`self.Delay between spawns`) 1.5))
    (else
      (`KismetSystemLibrary.K2_ClearAndInvalidateTimerHandle` (`self.SpawningTimer`))
      (`KismetSystemLibrary.PrintString` "Finished Spawning" true true (struct :`R` 1.0 :`G` 1.0 :`A` 1.0) 5.0))))

(event `Next Wave Setup`
  (`/Engine/EditorBlueprintResources/StandardMacros.DoOnce` false :!label _label
    (:`Completed`
      (bind _result (`/Engine/EditorBlueprintResources/StandardMacros.IncrementInt` (`self.Current wave`))
        (:`  `
          (if (== (`KismetArrayLibrary.Array_Length` (`self.Waves`)) _result)
            (bind _asgm_rabbit_smasher (cast `/Game/GameContent/Blueprints/GM_RabbitSmasher` (`GameplayStatics.GetGameMode`)))
            ;[1 1 1] mission complete
            (`/Game/GameContent/Blueprints/GM_RabbitSmasher.GameOverVictory` _asgm_rabbit_smasher)
            (else
              (`self.SetupWaveContents` _result)
              (set `self.Delay between spawns` (`KismetMathLibrary.Conv_IntToDouble` (+ _result 3)))
              ;[1 1 1] Time between waves
              (`KismetSystemLibrary.Delay` 6.0)
              (`self.Start Spawning`)
              (`|ExecutionSequence`
                (:`then_0`
                  (`KismetSystemLibrary.PrintString` "Next Wave" true true (struct :`R` 1.0 :`G` 1.0 :`A` 1.0) 5.0))
                (:`then_1`
                  (goto _label :!via `Reset`))))))))))

(event `Check if all dead?`
  (bind _newparam (`self.Check dead`))
  (if _newparam
    (`self.Next Wave Setup`)
    (`KismetSystemLibrary.PrintString` "Wave Over" true true (struct :`R` 1.0 :`G` 1.0 :`A` 1.0) 5.0)))

(fn `Check dead`
  (returns (NewParam :type Boolean))
  (if (not (> (`KismetArrayLibrary.Array_Length` (`self.Current wave enemies`)) 0))
    (bind _outactors (`GameplayStatics.GetAllActorsWithTag` "Enemy"))
    (return (== (`KismetArrayLibrary.Array_Length` _outactors) 1))))

(fn `SetupWaveContents`
  (params (Wave :type Integer))
  (bind _wave (break `/Game/GameContent/AI/RabbitBlueprints/F_EnemyWave` (`|GetArrayItem` (`self.Waves`) Wave)))
  (bind _keys (`BlueprintMapLibrary.Map_Keys` _wave))
  (for (_array_element _array_index) _keys
    (bind _values (`BlueprintMapLibrary.Map_Values` _wave))
    (for _ (range 1 (+ (`|GetArrayItem` _values _array_index) 1))
      (`KismetArrayLibrary.Array_Add` (`self.Current wave enemies`) _array_element)))
  (`KismetArrayLibrary.Array_Shuffle` (`self.Current wave enemies`)))

(fn `UserConstructionScript`)