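; Rabbit enemy NPC (T2) for a wave-based game that animates a mesh hop with a timeline and loops a positional walk sound.
; AnyDamage reduces health, spawning blood effects, and infers the killing weapon from the damage causer.
; Death awards player score, with a fists bonus or distance-scaled axe bonus, shown as a floating number.
; Both death and Destroyed notify BP_WaveController; an older flat-score death chain remains unconnected.
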(event `self.ReceiveBeginPlay`
  (`|ExecutionSequence`
    (:`then_0`
      (bind (_direction _newtrack_0) (`Timeline|Timeline_0` :!via `PlayFromStart`)
        (:`Update`
          (`SceneComponent.K2_SetRelativeLocation` (`self.StaticMesh`) (`KismetMathLibrary.MakeVector` 0.0 0.0 (`KismetMathLibrary.Lerp` 1.0 35.0 _newtrack_0)) false false))))
    (:`then_1`
      (`KismetSystemLibrary.Delay` 0.6 :!label _label)
      (`GameplayStatics.PlaySoundAtLocation` "/Game/GameContent/SoundEffects/RabbitWalk_Cue.RabbitWalk_Cue" (`self.K2_GetActorLocation`) (struct) 1.0 1.0 0.0 "/Game/GameContent/SoundEffects/AttenSetting.AttenSetting" null null null)
      (goto _label))))

(event `self.ReceiveDestroyed`
  (bind _returnvalue (`GameplayStatics.GetActorOfClass` "/Game/GameContent/AI/RabbitBlueprints/BP_WaveController.BP_WaveController_C"))
  (`/Game/GameContent/AI/RabbitBlueprints/BP_WaveController.Check if all dead?` _returnvalue self))

(event `self.ReceiveAnyDamage`
  (params (Damage :type "Float (single-precision)") (DamageType :type "DamageType Object Reference") (InstigatedBy :type "Controller Object Reference") (DamageCauser :type "Actor Object Reference"))
  (bind _returnvalue (`self.K2_GetActorLocation`))
  (bind _points_awarded_to_player (`self.Points awarded to player`))
  (bind _points_awarded_to_player_2 (`self.Points awarded to player`))
  (bind _output_get (set `self.Health` (- (`self.Health`) Damage)))
  (if (<= _output_get 0.0)
    (`|ExecutionSequence`
      (:`then_0`
        (bind _asbp_first_person_character (cast `/Game/FirstPerson/Blueprints/BP_FirstPersonCharacter` DamageCauser)
          (:`then`
            (if (`|EnumEquality` (`/Game/FirstPerson/Blueprints/BP_FirstPersonCharacter.Equipped item` _asbp_first_person_character) "NewEnumerator0")
              (set `self.Killed by` "NewEnumerator0")))
          (:`CastFailed`
            (bind _asbp_axe_projectile (cast `/Game/FirstPerson/Blueprints/BP_AxeProjectile` DamageCauser))
            (set `self.Start Location` (`/Game/FirstPerson/Blueprints/BP_AxeProjectile.Start location` _asbp_axe_projectile))
            (set `self.Killed by` "NewEnumerator2"))))
      (:`then_1`
        (`|SpawnActorFromClass` "/Game/UI/BP_FloatingNumber.BP_FloatingNumber_C" (`KismetMathLibrary.MakeTransform` _returnvalue (`KismetMathLibrary.FindLookAtRotation` _returnvalue (`self.K2_GetActorLocation` (`GameplayStatics.GetPlayerCharacter` 0)))) "Undefined" "OverrideRootScale" null (select `/Game/FirstPerson/Blueprints/Weapons` (`self.Killed by`) :`NewEnumerator0` (+ _points_awarded_to_player 50) :`NewEnumerator1` _points_awarded_to_player :`NewEnumerator2` (+ _points_awarded_to_player (`KismetMathLibrary.Round` (`KismetMathLibrary.MapRangeClamped` (`KismetMathLibrary.Vector_Distance` (`self.Start Location`) (`self.K2_GetActorLocation`)) 400.0 1800.0 0.0 50.0)))) null)
        (`NiagaraFunctionLibrary.SpawnSystemAtLocation` "/Game/GameContent/VFX/VX_BloodExplosion.VX_BloodExplosion" _returnvalue)
        (`GameplayStatics.PlaySoundAtLocation` "/Game/GameContent/SoundEffects/RabbitDeath.RabbitDeath" (`self.K2_GetActorLocation`) (struct) 1.2 1.0 0.0 "/Game/GameContent/SoundEffects/AttenSetting.AttenSetting" null null null)
        (bind _asbp_first_person_character_2 (cast `/Game/FirstPerson/Blueprints/BP_FirstPersonCharacter` (`GameplayStatics.GetPlayerCharacter` 0)))
        (set `/Game/FirstPerson/Blueprints/BP_FirstPersonCharacter.Score` (+ (`/Game/FirstPerson/Blueprints/BP_FirstPersonCharacter.Score` _asbp_first_person_character_2) (select `/Game/FirstPerson/Blueprints/Weapons` (`self.Killed by`) :`NewEnumerator0` (+ _points_awarded_to_player_2 50) :`NewEnumerator1` _points_awarded_to_player_2 :`NewEnumerator2` (+ _points_awarded_to_player_2 (`KismetMathLibrary.Round` (`KismetMathLibrary.MapRangeClamped` (`KismetMathLibrary.Vector_Distance` (`self.Start Location`) (`self.K2_GetActorLocation`)) 400.0 1800.0 0.0 50.0))))) _asbp_first_person_character_2)
        (bind _returnvalue_2 (`GameplayStatics.GetActorOfClass` "/Game/GameContent/AI/RabbitBlueprints/BP_WaveController.BP_WaveController_C"))
        (`/Game/GameContent/AI/RabbitBlueprints/BP_WaveController.Check if all dead?` _returnvalue_2 self)
        (`self.K2_DestroyActor`)))
    (else
      (`NiagaraFunctionLibrary.SpawnSystemAtLocation` "/Game/GameContent/VFX/VX_BloodExplosion_2.VX_BloodExplosion_2" (`self.K2_GetActorLocation`)))))

(fn `UserConstructionScript`)