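; Tier 3 rabbit enemy for the Rabbit Smasher game, which takes damage and awards points to the player when destroyed.
; BeginPlay caches the game mode, starts a Timeline that animates the mesh height as a hop and loops walk sounds on a delay.
; Damage spawns blood effects until health runs out and the actor is destroyed.
; Destroyed spawns a player-facing floating number, explosion and death sound, then adds score to the first-person character.
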(event `self.ReceiveDestroyed`
  (bind _returnvalue (`self.K2_GetActorLocation`))
  (`|SpawnActorFromClass` "/Game/UI/BP_FloatingNumber.BP_FloatingNumber_C" (`KismetMathLibrary.MakeTransform` _returnvalue (`KismetMathLibrary.FindLookAtRotation` _returnvalue (`self.K2_GetActorLocation` (`GameplayStatics.GetPlayerCharacter` 0)))) "Undefined" "OverrideRootScale" null (`self.Points awarded to player`) null)
  (`NiagaraFunctionLibrary.SpawnSystemAtLocation` "/Game/GameContent/VFX/VX_BloodExplosion.VX_BloodExplosion" _returnvalue)
  (`GameplayStatics.PlaySoundAtLocation` "/Game/GameContent/SoundEffects/RabbitDeath.RabbitDeath" (`self.K2_GetActorLocation`) (struct) 1.2 1.0 0.0 "/Game/GameContent/SoundEffects/AttenSetting.AttenSetting" null null null)
  (bind _asbp_first_person_character (cast `/Game/FirstPerson/Blueprints/BP_FirstPersonCharacter` (`GameplayStatics.GetPlayerCharacter` 0)))
  (set `/Game/FirstPerson/Blueprints/BP_FirstPersonCharacter.Score` (+ (`/Game/FirstPerson/Blueprints/BP_FirstPersonCharacter.Score` _asbp_first_person_character) (`self.Points awarded to player`)) _asbp_first_person_character))

(event `self.ReceiveBeginPlay`
  (bind _asgm_rabbit_smasher (cast `/Game/GameContent/Blueprints/GM_RabbitSmasher` (`GameplayStatics.GetGameMode`)))
  (set `self.As GM Rabbit Smasher` _asgm_rabbit_smasher)
  (`|ExecutionSequence`
    (:`then_0`
      (bind (_direction _newtrack_0) (`Timeline|Timeline_0` :!via `PlayFromStart`)
        (:`Update`
          (`SceneComponent.K2_SetRelativeLocation` (`self.StaticMesh`) (`KismetMathLibrary.MakeVector` 0.0 0.0 (`KismetMathLibrary.Lerp` 1.0 40.0 _newtrack_0)) false false))))
    (:`then_1`
      (`KismetSystemLibrary.Delay` 0.6 :!label _label)
      (`GameplayStatics.PlaySoundAtLocation` "/Game/GameContent/SoundEffects/RabbitWalk_Cue.RabbitWalk_Cue" (`self.K2_GetActorLocation`) (struct) 1.0 1.0 0.0 "/Game/GameContent/SoundEffects/AttenSetting.AttenSetting" null null null)
      (goto _label))))

(event `self.ReceiveAnyDamage`
  (params (Damage :type "Float (single-precision)") (DamageType :type "DamageType Object Reference") (InstigatedBy :type "Controller Object Reference") (DamageCauser :type "Actor Object Reference"))
  (bind _output_get (set `self.Health` (- (`self.Health`) Damage)))
  (if (<= _output_get 0.0)
    (`self.K2_DestroyActor`)
    (else
      (`NiagaraFunctionLibrary.SpawnSystemAtLocation` "/Game/GameContent/VFX/VX_BloodExplosion_2.VX_BloodExplosion_2" (`self.K2_GetActorLocation`)))))

(fn `UserConstructionScript`)