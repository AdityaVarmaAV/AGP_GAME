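; Farm level generator that builds an X by Y tile grid on BeginPlay for the RabbitSmasher game mode.
; Steps itself across the grid to record transforms and edges, then spawns fences and randomly picked edge spawn points, using bounded retries for spacing.
; Fills cells in random order with a ratio of crop tiles, then count-capped other tiles, flipping those past the middle index.
; Finally calls the game mode's GatherAllData and rebuilds navigation.
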(event `UpdateGameMode`
  (bind _asgm_rabbit_smasher (cast `/Game/GameContent/Blueprints/GM_RabbitSmasher` (`GameplayStatics.GetGameMode`)))
  (`/Game/GameContent/Blueprints/GM_RabbitSmasher.GatherAllData` _asgm_rabbit_smasher)
  (`KismetSystemLibrary.ExecuteConsoleCommand` "RebuildNavigation" null))

(event `GenerateTiles`
  (bind _d_tilesspawnrate (`self.D_TilesSpawnRate`))
  (bind _d_tilesspwancount (`self.D_TilesSpwanCount`))
  (bind _templocation (`self.tempLocation`))
  (bind _tilelocationindex (`self.TileLocationIndex`))
  (bind _output (`|GetArrayItem` (`self.TileLocationIndex`) (`self.RandomTempLoc_Index`)))
  (bind (_output_location _output_rotation _output_scale) (`KismetMathLibrary.BreakTransform` (`|GetArrayItem` (`self.TileLocations`) _output)))
  (bind _values (`BlueprintMapLibrary.Map_Values` (`self.D_TilesSpawnRate`)))
  (`self.ForLoopModified` 0 (`KismetArrayLibrary.Array_Length` _values)
    (:`LoopBody`
      (`KismetArrayLibrary.Array_Add` (`self.D_TilesSpwanCount`)))
    (:`Completed`
      (bind _output_get (set `self.TotalTiles` (`KismetArrayLibrary.Array_Length` _tilelocationindex)))
      (set `self.CenterTileIndex` (`|GetArrayItem` _tilelocationindex (/ _output_get 2)))
      (bind _output_get_2 (set `self.CropsTilesPercentage` (`KismetMathLibrary.Round` (* (* (`self.x`) (`self.y`)) (`self.CropTilesRatio`)))))
      (`self.ForLoopModified` 0 (`self.TotalTiles`)
        (:`LoopBody`
          (set `self.RandomTempLoc_Index` (`.OutIndex` (`KismetArrayLibrary.Array_Random` (`self.TileLocationIndex`))))
          (if (< _output (`self.CenterTileIndex`))
            (set `self.tempLocation` (`KismetMathLibrary.MakeTransform` _output_location _output_rotation _output_scale))
            (else
              (set `self.tempLocation` (`KismetMathLibrary.MakeTransform` (+ _output_location (1000.0 1000.0 0.0)) (struct :`Yaw` 180.0) _output_scale))))
          (if (< (`self.CropsTilesSpwanned`) _output_get_2)
            (`|SpawnActorFromClass` (`KismetArrayLibrary.Array_Random` (`self.CropTiles`)) _templocation "Undefined" "OverrideRootScale" null null)
            (bind _result (`/Engine/EditorBlueprintResources/StandardMacros.IncrementInt` (`self.CropsTilesSpwanned`))
              (:`  `
                (set `self.CropsTilesSpwanned` _result)))
            (else
              (bind _keys (`BlueprintMapLibrary.Map_Keys` _d_tilesspawnrate :!label _label))
              (bind _values_2 (`BlueprintMapLibrary.Map_Values` _d_tilesspawnrate))
              (bind _output_get_3 (set `self.tempIndex` (`.OutIndex` (`KismetArrayLibrary.Array_Random` _keys))))
              (bind _output_2 (`|GetArrayItem` _d_tilesspwancount _output_get_3))
              (if (< _output_2 (`|GetArrayItem` _values_2 _output_get_3))
                (bind _result_2 (`/Engine/EditorBlueprintResources/StandardMacros.IncrementInt` _output_2)
                  (:`  `
                    (`KismetArrayLibrary.Array_Set` _d_tilesspwancount (`self.tempIndex`) _result_2)
                    (`|SpawnActorFromClass` (`|GetArrayItem` _keys (`self.tempIndex`)) _templocation "Undefined" "OverrideRootScale" null null)))
                (else
                  (goto _label)))))
          (`KismetArrayLibrary.Array_Remove` (`self.TileLocationIndex`) (`self.RandomTempLoc_Index`)))
        (:`Completed`
          (`self.UpdateGameMode`))))))

(event `Generate_SpwanPoints`
  (bind _spwanpoints (`self.SpwanPoints`))
  (bind _tilelocations (`self.TileLocations`))
  (bind _randomsp (`self.RandomSP`))
  (bind _output_location (`KismetMathLibrary.BreakTransform` (`|GetArrayItem` _tilelocations (`self.RandomSP`))))
  (bind _output_get (set `self.SpwanPointsCount` (`KismetMathLibrary.RandomIntegerInRange` (`self.MinSpwanPoints`) (`self.MaxSpwanPoints`))))
  (for _ (range 1 (+ _output_get 1))
    (bind _output_get_2 (set `self.RandomSP` (`KismetArrayLibrary.Array_Random` (`self.ViableSpwanLocations`)) :!label _label_2))
    (if (== (`KismetArrayLibrary.Array_Length` (`self.SpwanPoints`)) 0)
      (`KismetArrayLibrary.Array_AddUnique` _spwanpoints _output_get_2)
      (`|SpawnActorFromClass` (`self.SpwanPointActor`) (`|GetArrayItem` (`self.TileLocations`) _output_get_2) "Undefined" "OverrideRootScale" null null)
      (`KismetArrayLibrary.Array_RemoveItem` (`self.ViableSpwanLocations`) (`self.RandomSP`))
      (else
        (for _array_element _spwanpoints
          (bind _output_location_2 (`KismetMathLibrary.BreakTransform` (`|GetArrayItem` _tilelocations _array_element)))
          (if (< (`KismetMathLibrary.Vector_Distance2D` _output_location_2 _output_location) 2000.0)
            (bind _result (`/Engine/EditorBlueprintResources/StandardMacros.IncrementInt` (`self.reloopcount`))
              (:`  `
                (bind _output_get_3 (set `self.reloopcount` _result))
                (if (< _output_get_3 (`KismetArrayLibrary.Array_Length` (`self.ViableSpwanLocations`)))
                  (goto _label_2))))))
        (`KismetArrayLibrary.Array_AddUnique` _spwanpoints _randomsp)
        (set `self.reloopcount` 0)
        (`|SpawnActorFromClass` (`self.SpwanPointActor`) (`|GetArrayItem` (`self.TileLocations`) _randomsp) "Undefined" "OverrideRootScale" null null)
        (`KismetArrayLibrary.Array_RemoveItem` (`self.ViableSpwanLocations`) (`self.RandomSP`)))))
  (`self.GenerateTiles`))

(event `GenerateFence`
  (bind _fencetype (`self.FenceType`))
  (bind _fence_map_x (`self.Fence_Map_X`))
  (bind _fencetype_2 (`self.FenceType`))
  (bind _fence_map_y (`self.Fence_Map_Y`))
  (`|ExecutionSequence`
    (:`then_0`
      (bind _index (`self.ForLoopModified` 0 (`BlueprintMapLibrary.Map_Length` _fence_map_x))
        (:`LoopBody`
          (bind _keys (`BlueprintMapLibrary.Map_Keys` _fence_map_x))
          (bind _values (`BlueprintMapLibrary.Map_Values` _fence_map_x))
          (if (`|GetArrayItem` _values _index)
            (bind _output (`|GetArrayItem` (`self.TileLocations`) (`|GetArrayItem` _keys _index)))
            (`|SpawnActorFromClass` (`|GetArrayItem` _fencetype_2) _output "Undefined" "OverrideRootScale" null null)
            (else
              (`|SpawnActorFromClass` (`|GetArrayItem` _fencetype_2 1) _output "Undefined" "OverrideRootScale" null null))))))
    (:`then_1`
      (bind _index_2 (`self.ForLoopModified` 0 (`BlueprintMapLibrary.Map_Length` _fence_map_y))
        (:`LoopBody`
          (bind _keys_2 (`BlueprintMapLibrary.Map_Keys` _fence_map_y))
          (bind _values_2 (`BlueprintMapLibrary.Map_Values` _fence_map_y))
          (if (`|GetArrayItem` _values_2 _index_2)
            (bind _output_2 (`|GetArrayItem` (`self.TileLocations`) (`|GetArrayItem` _keys_2 _index_2)))
            (`|SpawnActorFromClass` (`|GetArrayItem` _fencetype 2) _output_2 "Undefined" "OverrideRootScale" null null)
            (else
              (`|SpawnActorFromClass` (`|GetArrayItem` _fencetype 3) _output_2 "Undefined" "OverrideRootScale" null null))))
        (:`Completed`
          (`self.Generate_SpwanPoints`))))))

(event `StartGeneration`
  (bind (_returnvalue_x _returnvalue_y _returnvalue_z) (`KismetMathLibrary.BreakVector` (`self.K2_GetActorLocation`)))
  (bind _tilelocations (`self.TileLocations`))
  (`KismetArrayLibrary.Array_Clear` _tilelocations)
  (bind _index (`self.ForLoopModified` 0 (`self.x`))
    (:`LoopBody`
      (bind _index_2 (`self.ForLoopModified` 0 (`self.y`))
        (:`LoopBody`
          (bind _returnvalue (`KismetArrayLibrary.Array_AddUnique` _tilelocations (`self.GetTransform`)))
          (`self.K2_SetActorLocation` (+ (`self.K2_GetActorLocation`) (1000.0 0.0 0.0)))
          (`|ExecutionSequence`
            (:`then_0`
              (bind _returnvalue_2 (== _index 0))
              (if (or _returnvalue_2 (== _index (- (`self.x`) 1)))
                (`BlueprintMapLibrary.Map_Add` (`self.Fence_Map_X`) _returnvalue _returnvalue_2)
                (`KismetArrayLibrary.Array_AddUnique` (`self.ViableSpwanLocations`) _returnvalue :!label _label_3)))
            (:`then_1`
              (bind _returnvalue_3 (== _index_2 0))
              (if (or _returnvalue_3 (== _index_2 (- (`self.y`) 1)))
                (`BlueprintMapLibrary.Map_Add` (`self.Fence_Map_Y`) _returnvalue _returnvalue_3)
                (goto _label_3)))
            (:`then_2`
              (`KismetArrayLibrary.Array_AddUnique` (`self.TileLocationIndex`) _returnvalue))))
        (:`Completed`
          (`self.K2_SetActorLocation` (`KismetMathLibrary.MakeVector` (`self.Pos_Zero`) (+ _returnvalue_y 1000.0) _returnvalue_z)))))
    (:`Completed`
      (`self.GenerateFence`))))

(event `self.ReceiveBeginPlay`
  (`self.StartGeneration`))

(fn `UserConstructionScript`)