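; BP_BearTrap is a trap that immobilizes and damages enemies, and that the player can re-arm.
; An unused trap's DEATHBox overlap catches Enemy-tagged Characters, zeroing their walk speed, applying damage and marking the trap used.
; The original speed is saved but never restored.
; InteractBox enables input only while BP_FirstPersonCharacter overlaps it, letting Interact clear BeenUsed to reset the trap.
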(event `self.DEATH Box.OnComponentBeginOverlap`
  (params (OverlappedComponent :type "PrimitiveComponent Object Reference") (OtherActor :type "Actor Object Reference") (OtherComp :type "PrimitiveComponent Object Reference") (OtherBodyIndex :type Integer) (bFromSweep :type Boolean) (SweepResult :type "HitResult Structure (by ref)"))
  (if (`self.Been Used?`)
    _
    (elif (`self.ActorHasTag` OtherActor "Enemy")
      (bind _ascharacter (cast `Character` OtherActor)
        (:`then`
          (bind _charactermovement (`Character.CharacterMovement` _ascharacter))
          (set `self.Max Walk Speed` (`CharacterMovementComponent.MaxWalkSpeed` _charactermovement))
          (set `CharacterMovementComponent.MaxWalkSpeed` 0.0 _charactermovement)
          (set `self.Been Used?` true)
          (`GameplayStatics.ApplyDamage` OtherActor 30.0))
        (:`CastFailed`
          (`KismetSystemLibrary.PrintString` "Cast to character failed"))))))

(event `self.InteractBox.OnComponentBeginOverlap`
  (params (OverlappedComponent :type "PrimitiveComponent Object Reference") (OtherActor :type "Actor Object Reference") (OtherComp :type "PrimitiveComponent Object Reference") (OtherBodyIndex :type Integer) (bFromSweep :type Boolean) (SweepResult :type "HitResult Structure (by ref)"))
  (cast `/Game/FirstPerson/Blueprints/BP_FirstPersonCharacter` OtherActor)
  (`self.EnableInput` (`GameplayStatics.GetPlayerController` 0)))

(event `self.InteractBox.OnComponentEndOverlap`
  (params (OverlappedComponent :type "PrimitiveComponent Object Reference") (OtherActor :type "Actor Object Reference") (OtherComp :type "PrimitiveComponent Object Reference") (OtherBodyIndex :type Integer))
  (cast `/Game/FirstPerson/Blueprints/BP_FirstPersonCharacter` OtherActor)
  (`self.DisableInput` (`GameplayStatics.GetPlayerController` 0)))

(event `InputAction|Interact`
  (params (Key :type "Key Structure"))
  (:`Pressed`
    (set `self.Been Used?` false)))

(fn `UserConstructionScript`)